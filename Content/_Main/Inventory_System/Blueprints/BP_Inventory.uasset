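; BP_Inventory is a slot-based inventory that stores an item class and amount per slot, sized to AmountSlots on BeginPlay.
; Helper functions test whether a slot is empty, find the first empty slot, and return a slot's item info and amount.
; Items are held as soft class references: an invalid reference marks an empty slot, and item info is read from the class defaults.
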(event `self.ReceiveBeginPlay`
  (`KismetArrayLibrary.Array_Resize` (`self.slots`) (`self.amount_slots`)))

(fn `getItemInfoatIndex`
  (params (Index :type Integer))
  (returns (emtpy_slot :type Boolean) (item_info :type "/Game/_Main/Inventory_System/Blueprints/Structure/S_ItemInfo Structure") (amount :type Integer))
  (bind (_item_class _item_amount) (break `/Game/_Main/Inventory_System/Blueprints/Structure/S_InventorySlot` (`|GetArrayItem` (`self.slots`) Index)))
  (if (`KismetSystemLibrary.IsValidSoftClassReference` _item_class)
    (return false (defaults `Object` (`|ConvertAsset` _item_class)) _item_amount)
    (else
      (return true (struct) 0))))

(fn `isSlotEmpty`
  (params (index :type Integer))
  (returns (is_empty :type Boolean))
  (return (not (`KismetSystemLibrary.IsValidSoftClassReference` (`.item_class_4_46F7DE584A7958E82ADA8688EF6D2240` (break `/Game/_Main/Inventory_System/Blueprints/Structure/S_InventorySlot` (`|GetArrayItem` (`self.slots`) index)))))))

(fn `searchEmptySlot`
  (returns (success :type Boolean) (index :type Integer))
  (locals (localBool :type Boolean) (localIndex :type Integer))
  (for (_array_element _array_index) (`self.slots`)
    (if (not (`KismetSystemLibrary.IsValidSoftClassReference` (`.item_class_4_46F7DE584A7958E82ADA8688EF6D2240` (break `/Game/_Main/Inventory_System/Blueprints/Structure/S_InventorySlot` _array_element))))
      (set `local.localBool` true)
      (set `local.localIndex` _array_index)
      (break)))
  (return (`local.localBool`) (`local.localIndex`)))

(fn `UserConstructionScript`)