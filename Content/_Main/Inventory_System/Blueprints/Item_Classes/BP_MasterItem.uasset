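; BP_MasterItem is an item actor in the inventory system, apparently the base item class, with built-in medkit use logic.
; Its onUse event acts only when the item's name matches MedkitCheck, adding a fixed, unclamped amount to the first-person character's CurrentHealth.
; It then removes one unit at its Index from the Inventory and destroys itself if that removal succeeds.
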(event `onUse`
  (if (`KismetTextLibrary.EqualEqual_TextText` (`.name_2_06991B924938E054623436B94D9D3F8E` (break `/Game/_Main/Inventory_System/Blueprints/Structure/S_ItemInfo` (`self.Item_Information`))) (`KismetTextLibrary.Conv_StringToText` (`self.medkit_check`)))
    (bind _asbp_first_person_character (cast `/Game/_Main/Blueprints/BP_FirstPersonCharacter` (`GameplayStatics.GetPlayerCharacter` 0)))
    (set `/Game/_Main/Blueprints/BP_FirstPersonCharacter.Current_Health` (+ (`/Game/_Main/Blueprints/BP_FirstPersonCharacter.Current_Health` _asbp_first_person_character) 30.0) _asbp_first_person_character)
    (bind _success (`/Game/_Main/Inventory_System/Blueprints/BP_Inventory.Remove Item at Index` (`self.Inventory`) (`self.index`) 1))
    (if _success
      (`self.K2_DestroyActor`))))

(fn `UserConstructionScript`)