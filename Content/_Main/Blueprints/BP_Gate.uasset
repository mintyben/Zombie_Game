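; Gate actor that sends the player down one floor, from Floor14 through Floor1, when BP_Character enters its Box trigger.
; A hardcoded chain of equality checks on the character's CurrentFloor picks the level name to open.
; Each matched branch calls Open Level, then decrements CurrentFloor on that character instance.
; The check for floor 1 is an empty end point, so nothing happens there.
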(event `self.Box.OnComponentBeginOverlap`
  (params (OverlappedComponent :type "PrimitiveComponent Object Reference") (OtherActor :type "Actor Object Reference") (OtherComp :type "PrimitiveComponent Object Reference") (OtherBodyIndex :type Integer) (bFromSweep :type Boolean) (SweepResult :type "HitResult Structure (by ref)"))
  (bind _asbp_character (cast `/Game/PistolAnimation/System/Blueprints/BP_Character` OtherActor))
  (bind _currentfloor (`/Game/PistolAnimation/System/Blueprints/BP_Character.CurrentFloor` _asbp_character))
  (if (== _currentfloor 15.0)
    (`GameplayStatics.OpenLevel` "Floor14")
    (set `/Game/PistolAnimation/System/Blueprints/BP_Character.CurrentFloor` (- _currentfloor 1.0) _asbp_character :!label _label)
    (elif (== _currentfloor 14.0)
      (`GameplayStatics.OpenLevel` "Floor13")
      (goto _label)
      (elif (== _currentfloor 13.0)
        (`GameplayStatics.OpenLevel` "Floor12")
        (goto _label)
        (elif (== _currentfloor 12.0)
          (`GameplayStatics.OpenLevel` "Floor11")
          (goto _label)
          (elif (== _currentfloor 11.0)
            (`GameplayStatics.OpenLevel` "Floor10")
            (goto _label)
            (elif (== _currentfloor 10.0)
              (`GameplayStatics.OpenLevel` "Floor9")
              (goto _label)
              (elif (== _currentfloor 9.0)
                (`GameplayStatics.OpenLevel` "Floor8")
                (goto _label)
                (elif (== _currentfloor 8.0)
                  (`GameplayStatics.OpenLevel` "Floor7")
                  (goto _label)
                  (elif (== _currentfloor 7.0)
                    (`GameplayStatics.OpenLevel` "Floor6")
                    (goto _label)
                    (elif (== _currentfloor 6.0)
                      (`GameplayStatics.OpenLevel` "Floor5")
                      (goto _label)
                      (elif (== _currentfloor 5.0)
                        (`GameplayStatics.OpenLevel` "Floor4")
                        (goto _label)
                        (elif (== _currentfloor 4.0)
                          (`GameplayStatics.OpenLevel` "Floor3")
                          (goto _label)
                          (elif (== _currentfloor 3.0)
                            (`GameplayStatics.OpenLevel` "Floor2")
                            (goto _label)
                            (elif (== _currentfloor 2.0)
                              (`GameplayStatics.OpenLevel` "Floor1")
                              (goto _label)
                              (elif (== _currentfloor 1.0)
                                _))))))))))))))))

(fn `UserConstructionScript`)