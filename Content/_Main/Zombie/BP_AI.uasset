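; Zombie AI character that takes damage, dies and performs a melee attack.
; Incoming damage, except from ZombieREF, lowers Health; at zero the mesh simulates physics, movement is disabled and IsDead blocks further attacks.
; Attack plays a montage whose notify sphere-traces for pawns and damages the hit actor.
; The trace starts at the actor, but its end is a forward offset from world origin, not from the actor.
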(event `self.ReceiveAnyDamage`
  (params (Damage :type "Float (single-precision)") (DamageType :type "DamageType Object Reference") (InstigatedBy :type "Controller Object Reference") (DamageCauser :type "Actor Object Reference"))
  ;[1 1 1] AI Taking Damage
  (if (not (== DamageCauser (`self.Zombie_REF`)))
    (set `self.health` (- (`self.health`) Damage))
    (if (<= (`self.health`) 0.0)
      (`PrimitiveComponent.SetSimulatePhysics` (`self.Mesh`) true)
      (set `self.isDead` true)
      (`CharacterMovementComponent.DisableMovement` (`self.CharacterMovement`)))))

(event `/Game/_Main/Zombie/BPI_AI.Attack`
  ;[1 1 1] AI Attack Player
  (if (not (`self.isDead`))
    (`|PlayMontage` (`self.Mesh`) "/Game/Characters/Mannequins/Animations/Attack_Montage.Attack_Montage"
      (:`OnNotifyBegin`
        (bind (_outhit _returnvalue) (`KismetSystemLibrary.SphereTraceSingleForObjects` (`self.K2_GetActorLocation`) (+ (0.0 0.0 0.0) (* (`KismetMathLibrary.GetForwardVector` (`self.K2_GetActorRotation`)) 170.0)) 150.0 (`|MakeArray` "ObjectTypeQuery3" :!type "EObjectTypeQuery Enum")))
        (if _returnvalue
          (`GameplayStatics.ApplyDamage` (`.HitActor` (`GameplayStatics.BreakHitResult` _outhit)) 10.0))))))

(fn `UserConstructionScript`)