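; Zombie AI controller that runs the BT_AI behavior tree and reports perception of the player to it.
; On begin play it starts the tree, then listens for AI perception updates on actors tagged Player.
; Both the sensed and lost branches set the isSeeingPlayer blackboard key to true, so this controller never clears it.
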(event `self.ReceiveBeginPlay`
  (`self.RunBehaviorTree` "/Game/_Main/Zombie/BT_AI.BT_AI"))

(event `self.AIPerception.OnTargetPerceptionUpdated`
  (params (Actor :type "Actor Object Reference") (Stimulus :type "AIStimulus Structure"))
  (if (`self.ActorHasTag` Actor "Player")
    (if (`.bSuccessfullySensed` (break `AIStimulus` Stimulus))
      (`BlackboardComponent.SetValueAsBool` (`AIBlueprintHelperLibrary.GetBlackboard` null) "isSeeingPlayer" true)
      (else
        (`BlackboardComponent.SetValueAsBool` (`AIBlueprintHelperLibrary.GetBlackboard` null) "isSeeingPlayer" true)))))

(fn `UserConstructionScript`)